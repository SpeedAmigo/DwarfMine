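; Enemy AI character that chases the first-person player or cart entering its trigger and fires at them.
; Tick issues AIMoveTo toward the first entry in the Target array, then fires after a delay; a second trigger's end overlap removes targets.
; Fire uses a forward line trace, damaging only the player character.
; TakeDamage updates a player-facing health-bar widget or destroys the enemy at zero HP.
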(event `self.ReceiveBeginPlay`
  (set `CharacterMovementComponent.MaxWalkSpeed` (`self.speed`) (`self.CharacterMovement`)))

(event `self.ReceiveTick`
  (params (DeltaSeconds :type "Float (single-precision)"))
  (bind _target (`self.target`))
  (`self.WidgetLookAtPlayer`)
  (if (< 0 (`KismetArrayLibrary.Array_Length` _target))
    (`|AIMoveTo` self (0.0 0.0 0.0) (`|GetArrayItem` _target) 200.0
      (:`OnSuccess`
        (`KismetSystemLibrary.Delay` (`self.fireRate`))
        (`self.fire` 10 1000.0)))))

(event `self.Trigger.OnComponentBeginOverlap`
  (params (OverlappedComponent :type "PrimitiveComponent Object Reference") (OtherActor :type "Actor Object Reference") (OtherComp :type "PrimitiveComponent Object Reference") (OtherBodyIndex :type Integer) (bFromSweep :type Boolean) (SweepResult :type "HitResult Structure (by ref)"))
  (bind _target (`self.target`))
  (bind _asbp_first_person_character (cast `/Game/FirstPerson/Blueprints/BP_FirstPersonCharacter` OtherActor)
    (:`then`
      (`KismetArrayLibrary.Array_Add` _target _asbp_first_person_character))
    (:`CastFailed`
      (bind _asbp_cart (cast `/Game/Blueprints/BP_Cart` OtherActor))
      (`KismetArrayLibrary.Array_Add` _target _asbp_cart))))

(event `WidgetLookAtPlayer`
  (`SceneComponent.K2_SetWorldRotation` (`self.Widget`) (`KismetMathLibrary.FindLookAtRotation` (`self.K2_GetActorLocation`) (`self.K2_GetActorLocation` (`GameplayStatics.GetPlayerPawn` 0))) false false))

(event `self.Trigger1.OnComponentEndOverlap`
  (params (OverlappedComponent :type "PrimitiveComponent Object Reference") (OtherActor :type "Actor Object Reference") (OtherComp :type "PrimitiveComponent Object Reference") (OtherBodyIndex :type Integer))
  (`KismetArrayLibrary.Array_RemoveItem` (`self.target`) OtherActor))

(fn `fire`
  (params (damage :type Integer) (distance :type "Float (double-precision)"))
  (bind _returnvalue (`self.K2_GetActorLocation`))
  (set `self.isAttacking` true)
  (bind _outhits (`KismetSystemLibrary.LineTraceMulti` _returnvalue (+ _returnvalue (* (`KismetMathLibrary.GetForwardVector` (`.OutRotation` (`self.GetActorEyesViewPoint`))) distance)) "TraceTypeQuery1"))
  (bind _asbp_first_person_character (cast `/Game/FirstPerson/Blueprints/BP_FirstPersonCharacter` (`.HitActor` (`GameplayStatics.BreakHitResult` (`|GetArrayItem` _outhits)))))
  (`/Game/FirstPerson/Blueprints/BP_FirstPersonCharacter.TakeDamage` _asbp_first_person_character damage)
  (set `self.isAttacking` false))

(fn `TakeDamage`
  (params (Damage :type Integer))
  (bind _output_get (set `self.HP` (- (stale _output_get) Damage)))
  (if (<= _output_get 0)
    (`self.K2_DestroyActor`)
    (else
      (bind _asenemy_widget (cast `/Game/Widgets/EnemyWidget` (`WidgetComponent.GetWidget` (`self.Widget`))))
      (`ProgressBar.SetPercent` (`/Game/Widgets/EnemyWidget.ProgressBar_0` _asenemy_widget) (/ (`KismetMathLibrary.Conv_IntToDouble` (`self.HP`)) 100.0)))))

(fn `UserConstructionScript`)