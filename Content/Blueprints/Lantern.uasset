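; Lantern Blueprint that makes its point light flicker continuously.
; Each Tick adds delta time to an elapsed clock, which is scaled by FlickerSpeed and fed into 1D Perlin noise for a smooth, irregular pattern.
; The noise is remapped to a fixed brightness range, multiplied by Intensity and applied as the light's intensity.
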(event `self.ReceiveTick`
  (params (DeltaSeconds :type "Float (single-precision)"))
  (bind _output_get (set `self.ElapsedTime` (+ (`self.ElapsedTime`) DeltaSeconds)))
  (`LightComponent.SetIntensity` (`self.PointLight`) (* (`KismetMathLibrary.MapRangeClamped` (`KismetMathLibrary.PerlinNoise1D` (* _output_get (`self.FlickerSpeed`))) -1.0 1.0 3000.0 7000.0) (`self.Intensity`))))

(fn `UserConstructionScript`)