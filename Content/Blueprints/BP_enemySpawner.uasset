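; Enemy spawner actor that creates BP_AI actors at its own transform in timed waves.
; From BeginPlay it runs an endless Delay loop, spawning a Count-driven batch on each pass while CanSpawn is true.
; Spawned is never decremented here, so Limit caps the total spawned rather than the number alive, and the loop keeps ticking after the cap.
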(event `self.ReceiveBeginPlay`
  (if (`self.canSpawn`) :!label _label
    (for _ (range (+ (`self.count`) 1))
      (if (< (`self.spawned`) (`self.limit`))
        (`|SpawnActorFromClass` "/Game/Blueprints/BP_AI.BP_AI_C" (`self.GetTransform`) "Undefined" "MultiplyWithRoot" null null)
        (bind _output_get (set `self.spawned` (+ (stale _output_get) 1))))))
  (`KismetSystemLibrary.Delay` (`self.delay`))
  (goto _label))

(fn `UserConstructionScript`)