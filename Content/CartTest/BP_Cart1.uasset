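; BP_Cart1 is a cart actor that moves a cube along a spline while something overlaps its collision sphere.
; Sphere begin and end overlap events toggle a single flag without filtering the overlapping actor, and Tick calls MoveCart while it is set.
; MoveCart advances the spline distance by speed and delta time, without clamping or wrapping, then applies that point's local transform, without scale, to the cube.
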(event `self.CollisionSphere.OnComponentBeginOverlap`
  (params (OverlappedComponent :type "PrimitiveComponent Object Reference") (OtherActor :type "Actor Object Reference") (OtherComp :type "PrimitiveComponent Object Reference") (OtherBodyIndex :type Integer) (bFromSweep :type Boolean) (SweepResult :type "HitResult Structure (by ref)"))
  (set `self.isOverlapping` true))

(event `MoveCart`
  (params (`Delta Seconds` :type "Float (double-precision)"))
  (set `self.SplineDistance` (+ (* `Delta Seconds` (`self.MoveSpeed`)) (`self.SplineDistance`)))
  (`SceneComponent.K2_SetRelativeTransform` (`self.Cube`) (`SplineComponent.GetTransformAtDistanceAlongSpline` (`self.Spline`) (`self.SplineDistance`) "Local" false) false false))

(event `self.CollisionSphere.OnComponentEndOverlap`
  (params (OverlappedComponent :type "PrimitiveComponent Object Reference") (OtherActor :type "Actor Object Reference") (OtherComp :type "PrimitiveComponent Object Reference") (OtherBodyIndex :type Integer))
  (set `self.isOverlapping` false))

(event `self.ReceiveTick`
  (params (DeltaSeconds :type "Float (single-precision)"))
  (if (`self.isOverlapping`)
    (`self.MoveCart` DeltaSeconds)))

(fn `UserConstructionScript`)