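; BP_Cart is a cart that travels along a spline track while its collision sphere is overlapped.
; The construction script builds the track from one spline mesh component per spline segment.
; Tick advances the distance by MoveSpeed and sets Cart1's relative transform from the spline, with no end clamp or wrap.
; Movement plays random sounds back to back, and ending overlap stops both cart and audio.
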(event `self.CollisionSphere.OnComponentBeginOverlap`
  (params (OverlappedComponent :type "PrimitiveComponent Object Reference") (OtherActor :type "Actor Object Reference") (OtherComp :type "PrimitiveComponent Object Reference") (OtherBodyIndex :type Integer) (bFromSweep :type Boolean) (SweepResult :type "HitResult Structure (by ref)"))
  (set `self.isOverlapping` true))

(event `MoveCart`
  (params (`Delta Seconds` :type "Float (double-precision)"))
  (bind _sounds (`self.Sounds`))
  (bind _audio (`self.Audio`))
  (set `self.SplineDistance` (+ (* `Delta Seconds` (`self.MoveSpeed`)) (`self.SplineDistance`)))
  (`SceneComponent.K2_SetRelativeTransform` (`self.Cart1`) (`SplineComponent.GetTransformAtDistanceAlongSpline` (`self.Spline`) (`self.SplineDistance`) "Local" false) false false)
  (if (not (`AudioComponent.IsPlaying` _audio))
    (`AudioComponent.SetSound` _audio (`|GetArrayItem` _sounds (`KismetMathLibrary.RandomInteger` (`KismetArrayLibrary.Array_Length` _sounds))))
    (`AudioComponent.Play` _audio 0.0)))

(event `self.CollisionSphere.OnComponentEndOverlap`
  (params (OverlappedComponent :type "PrimitiveComponent Object Reference") (OtherActor :type "Actor Object Reference") (OtherComp :type "PrimitiveComponent Object Reference") (OtherBodyIndex :type Integer))
  (set `self.isOverlapping` false)
  (`AudioComponent.Stop` (`self.Audio`)))

(event `self.ReceiveTick`
  (params (DeltaSeconds :type "Float (single-precision)"))
  (if (`self.isOverlapping`)
    (`self.MoveCart` DeltaSeconds)))

(event `self.ReceiveBeginPlay`
  (`self.MoveCart` 0.0)
  (`AudioComponent.Stop` (`self.Audio`)))

(fn `UserConstructionScript`
  (bind _spline (`self.Spline`))
  (for _index (range (+ (- (`SplineComponent.GetNumberOfSplinePoints` (`self.Spline`)) 2) 1))
    (bind _returnvalue (`AddComponent|NODE_AddSplineMeshComponent-1`))
    (`SplineMeshComponent.SetForwardAxis` _returnvalue "X" true)
    (bind _returnvalue_2 (+ _index 1))
    (`SplineMeshComponent.SetStartAndEnd` _returnvalue (`SplineComponent.GetLocationAtSplinePoint` _spline _index "Local") (`SplineComponent.GetTangentAtSplinePoint` _spline _index "Local") (`SplineComponent.GetLocationAtSplinePoint` _spline _returnvalue_2 "Local") (`SplineComponent.GetTangentAtSplinePoint` _spline _returnvalue_2 "Local") false)))