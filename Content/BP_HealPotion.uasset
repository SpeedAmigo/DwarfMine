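; Health potion pickup that applies its HealthValue when its Collider overlap passes a check against player controller 0.
; AddHealth finds the first BP_FirstPersonCharacter in the level and passes a value derived from HealthValue to its TakeDamage, reusing the damage path for healing.
; The overlap compares the other actor to the controller itself, not its pawn; on a match it also plays a 2D sound and destroys the potion.
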(event `AddHealth`
  (bind _outactors (`GameplayStatics.GetAllActorsOfClass` "/Game/FirstPerson/Blueprints/BP_FirstPersonCharacter.BP_FirstPersonCharacter_C"))
  (bind _result (`/Engine/EditorBlueprintResources/StandardMacros.NegateInt` (`self.HealthValue`))
    (:`  `
      (`/Game/FirstPerson/Blueprints/BP_FirstPersonCharacter.TakeDamage` (`|GetArrayItem` _outactors) _result))))

(event `self.Collider.OnComponentBeginOverlap`
  (params (OverlappedComponent :type "PrimitiveComponent Object Reference") (OtherActor :type "Actor Object Reference") (OtherComp :type "PrimitiveComponent Object Reference") (OtherBodyIndex :type Integer) (bFromSweep :type Boolean) (SweepResult :type "HitResult Structure (by ref)"))
  (if (== OtherActor (`GameplayStatics.GetPlayerController` 0))
    (`self.AddHealth`)
    (`GameplayStatics.PlaySound2D` "/Game/Sounds/UI_Animate_Zap_Subtle_Disappear_stereo.UI_Animate_Zap_Subtle_Disappear_stereo" 1.0 1.0 0.0 null null)
    (`self.K2_DestroyActor`)))

(fn `UserConstructionScript`)